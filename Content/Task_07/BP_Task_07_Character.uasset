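; Player character that grabs physics objects with a camera line trace while the left mouse button is held.
; A physics constraint links the hit component to a Sphere anchor, which the mouse wheel moves, and the held object ignores Pawn collision until release.
; A cable attaches to the grabbed actor as a visible tether, with Tick stepping its end offset inward and printing it.
; Release breaks the constraint and hides the cable.
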(event `EnhancedInput|/Game/Basic/Input/IA_LeftMouse`
  (params (ActionValue :type Boolean) (ElapsedSeconds :type "Float (double-precision)") (TriggeredSeconds :type "Float (double-precision)") (InputAction :type "InputAction Object Reference" :default "/Game/Basic/Input/IA_LeftMouse.IA_LeftMouse"))
  (:`Triggered`
    (`/Engine/EditorBlueprintResources/StandardMacros.IsValid` (`self.HeldObject`)
      (:`Is Not Valid`
        (bind (_hitresult _hit) (`self.TraceObjects`))
        (if _hit
          (`self.GrabObject` _hitresult)
          (`self.AttachCable` _hitresult)))))
  (:`Completed`
    (`self.DropObject`)
    (`self.DetachCable`)))

(event `EnhancedInput|/Game/Basic/Input/IA_MouseWheel`
  (params (ActionValue :type "Float (double-precision)") (ElapsedSeconds :type "Float (double-precision)") (TriggeredSeconds :type "Float (double-precision)") (InputAction :type "InputAction Object Reference" :default "/Game/Basic/Input/IA_MouseWheel.IA_MouseWheel"))
  (:`Triggered`
    (`SceneComponent.K2_SetRelativeLocation` (`self.Sphere`) (+ (`SceneComponent.RelativeLocation` (`self.Sphere`)) (* (`self.ObjectMoveDistance`) ActionValue)) false false)))

(event `self.ReceiveTick`
  (params (DeltaSeconds :type "Float (single-precision)"))
  (bind _cable (`self.Cable`))
  (bind _endlocation (`CableComponent.EndLocation` _cable))
  (`/Engine/EditorBlueprintResources/StandardMacros.IsValid` (`self.HeldObject`)
    (:`Is Valid`
      (if (> (`KismetMathLibrary.VSize` _endlocation) 10.0)
        (bind _output_get (set `CableComponent.EndLocation` (+ _endlocation (5.0 0.0 0.0)) _cable))
        (`KismetSystemLibrary.PrintString` (`KismetStringLibrary.Conv_VectorToString` _output_get))))))

(fn `AttachCable`
  (params (HItResult :type "HitResult Structure"))
  (bind (_bblockinghit _binitialoverlap _time _distance _location _impactpoint _normal _impactnormal _physmat _hitactor) (`GameplayStatics.BreakHitResult` HItResult))
  (bind _cable (`self.Cable`))
  (bind _cable_2 (`self.Cable`))
  (`SceneComponent.SetHiddenInGame` _cable_2 false false)
  (bind _output_get (set `CableComponent.CableLength` (`self.GetDistanceTo` _hitactor) _cable_2))
  (set `CableComponent.EndLocation` (`KismetMathLibrary.MakeVector` (/ _output_get -2.0)) _cable)
  (set `CableComponent.bAttachEnd` true _cable)
  (`CableComponent.SetAttachEndTo` _cable_2 _hitactor "None" "None")
  (`PrimitiveComponent.SetPhysicsLinearVelocity` (`StaticMeshActor.StaticMeshComponent` (cast `StaticMeshActor` _hitactor :!pure true)) (1.0 1.0 0.0) false "None"))

(fn `DetachCable`
  (bind _cable (`self.Cable`))
  (set `CableComponent.CableLength` 10.0 _cable)
  (set `CableComponent.bAttachEnd` false _cable)
  (`SceneComponent.SetHiddenInGame` _cable true false))

(fn `DropObject`
  (bind _heldobject (`self.HeldObject`))
  (`PhysicsConstraintComponent.BreakConstraint` (`self.GrabConstrait`))
  (`/Engine/EditorBlueprintResources/StandardMacros.IsValid` _heldobject
    (:`Is Valid`
      (`PrimitiveComponent.SetCollisionResponseToChannel` _heldobject "ECC_Pawn" "ECR_Block")
      (set `self.HeldObject` null))))

(fn `GrabObject`
  (params (HitResult :type "HitResult Structure"))
  (bind (_bblockinghit _binitialoverlap _time _distance _location _impactpoint _normal _impactnormal _physmat _hitactor _hitcomponent _hitbonename) (`GameplayStatics.BreakHitResult` HitResult))
  (`SceneComponent.K2_SetWorldLocation` (`self.Sphere`) _location false true)
  (`PhysicsConstraintComponent.SetConstrainedComponents` (`self.GrabConstrait`) (`self.Sphere`) "None" _hitcomponent _hitbonename)
  (`PrimitiveComponent.SetCollisionResponseToChannel` _hitcomponent "ECC_Pawn" "ECR_Ignore")
  (set `self.HeldObject` _hitcomponent))

(fn `TraceObjects`
  (returns (HitResult :type "HitResult Structure") (Hit :type Boolean))
  (bind _camera (`self.Camera`))
  (bind _returnvalue (`SceneComponent.K2_GetComponentLocation` _camera))
  (bind (_outhit _returnvalue_2) (`KismetSystemLibrary.LineTraceSingleForObjects` :`Start` _returnvalue :`End` (+ _returnvalue (* (`SceneComponent.GetForwardVector` _camera) 1000.0)) :`ObjectTypes` (`|MakeArray` "ObjectTypeQuery4" :!type "EObjectTypeQuery Enum") :`DrawDebugType` "ForOneFrame" :`DrawTime` 0.0))
  (return _outhit _returnvalue_2))

(fn `UserConstructionScript`)