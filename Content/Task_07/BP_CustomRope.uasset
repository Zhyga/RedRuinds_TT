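; BP_CustomRope is an actor that builds a physics rope at BeginPlay from a chain of sphere meshes spawned along local X.
; A requested length sets the segment count, and each step adds a simulated sphere with gravity off and all collision responses ignored.
; Each sphere gets a physics constraint with locked linear axes, offset along X and linking it to the previous sphere in the stored array.
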(event `self.ReceiveBeginPlay`
  (`self.SetStartLenght` 1000.0))

(event `SetStartLenght`
  (params (Length :type "Float (double-precision)"))
  (bind _output_get (set `self.AmountOfSpheres` (/ Length 25.0)))
  (for _ (range (+ (`KismetMathLibrary.FFloor` _output_get) 1))
    (`self.SpawnSpheres`)
    (`self.SpawnConstraits`)))

(fn `SpawnConstraits`
  (bind _newvar (`self.NewVar`))
  (bind _lastspawnedsphere (`self.LastSpawnedSphere`))
  (bind _lastspawnedconstrait (`self.LastSpawnedConstrait`))
  (bind _returnvalue (`AddComponent|NODE_AddPhysicsConstraintComponent-0` :`bManualAttachment` true))
  (set `self.LastSpawnedConstrait` _returnvalue)
  (`PhysicsConstraintComponent.SetDisableCollision` _returnvalue true)
  (`PhysicsConstraintComponent.SetLinearXLimit` _returnvalue "LCM_Locked" 20.0)
  (`PhysicsConstraintComponent.SetLinearYLimit` _returnvalue "LCM_Locked" 20.0)
  (`PhysicsConstraintComponent.SetLinearZLimit` _returnvalue "LCM_Locked" 20.0)
  (`PhysicsConstraintComponent.SetAngularDriveMode` _returnvalue "TwistAndSwing")
  (`SceneComponent.K2_AttachToComponent` (`self.LastSpawnedConstrait`) (`self.LastSpawnedSphere`) "None" "KeepRelative" "KeepRelative" "KeepRelative" true)
  (`SceneComponent.K2_AddLocalOffset` _lastspawnedconstrait (25.0 0.0 0.0) false false)
  (`PhysicsConstraintComponent.SetConstrainedComponents` _lastspawnedconstrait _lastspawnedsphere "None" (`|GetArrayItem` _newvar (- (`KismetArrayLibrary.Array_Find` _newvar _lastspawnedsphere) 1)) "None"))

(fn `SpawnSpheres`
  (bind (_lastsphererelativelocation_x _lastsphererelativelocation_y _lastsphererelativelocation_z) (`KismetMathLibrary.BreakVector` (`self.LastSphereRelativeLocation`)))
  (bind _returnvalue (`AddComponent|NODE_AddStaticMeshComponent-0` :`RelativeTransform` (`KismetMathLibrary.MakeTransform` (`self.LastSphereRelativeLocation`))))
  (bind _output_get (set `self.LastSpawnedSphere` _returnvalue))
  (`KismetArrayLibrary.Array_Add` (`self.NewVar`) _output_get)
  (`StaticMeshComponent.SetStaticMesh` _returnvalue "/Engine/EditorMeshes/EditorSphere.EditorSphere")
  (`PrimitiveComponent.SetSimulatePhysics` _returnvalue true)
  (`PrimitiveComponent.SetCollisionObjectType` _returnvalue "ECC_PhysicsBody")
  (`PrimitiveComponent.SetCollisionResponseToAllChannels` _returnvalue "ECR_Ignore")
  (`PrimitiveComponent.SetEnableGravity` _returnvalue false)
  (set `self.LastSphereRelativeLocation` (`KismetMathLibrary.MakeVector` (+ _lastsphererelativelocation_x 50.0) _lastsphererelativelocation_y _lastsphererelativelocation_z)))

(fn `UserConstructionScript`)