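; Player character that rides a looping BP_Trajectory spline at its own height and throws physics balls from the camera.
; Tick advances distance along the spline, with inputs raising or lowering speed.
; Holding left mouse draws a projectile arc computed from velocity and gravity at sampled times, sphere-tracing to those points to place a hit preview.
; Releasing it spawns BP_PhysicBall with velocity along camera forward.
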(event `self.ReceiveBeginPlay`
  (bind (_returnvalue_x _returnvalue_y _returnvalue_z) (`KismetMathLibrary.BreakVector` (`self.K2_GetActorLocation`)))
  ;[1 1 1] Finding first spline point and setting character location to it
  (bind _returnvalue (`GameplayStatics.GetActorOfClass` "/Game/Task_05/BP_Trajectory.BP_Trajectory_C"))
  (bind _output_get (set `self.Trajectory` _returnvalue))
  (bind (_returnvalue_x_2 _returnvalue_y_2) (`KismetMathLibrary.BreakVector` (+ (`self.K2_GetActorLocation` _output_get) (`.Position` (break `SplinePoint` (`SplineComponent.GetSplinePointAt` (`/Game/Task_05/BP_Trajectory.Spline` _output_get) 0 "Local"))))))
  (`self.K2_SetActorLocation` (`KismetMathLibrary.MakeVector` _returnvalue_x_2 _returnvalue_y_2 _returnvalue_z)))

(event `self.ReceiveTick`
  (params (DeltaSeconds :type "Float (single-precision)"))
  (bind (_returnvalue_x _returnvalue_y _returnvalue_z) (`KismetMathLibrary.BreakVector` (`self.K2_GetActorLocation`)))
  (bind (_returnvalue_location _returnvalue_rotation) (`KismetMathLibrary.BreakTransform` (`SplineComponent.GetTransformAtDistanceAlongSpline` (`/Game/Task_05/BP_Trajectory.Spline` (`self.Trajectory`)) (`self.DistanceAlongSpline`) "Local" false)))
  (bind (_returnvalue_x_2 _returnvalue_y_2) (`KismetMathLibrary.BreakVector` (+ (`self.K2_GetActorLocation` (`self.Trajectory`)) _returnvalue_location)))
  ;[1 1 1] Moveing Character along the spline
  (set `self.DistanceAlongSpline` (+ (* DeltaSeconds (`self.MoveSpeedAlongSpline`)) (`self.DistanceAlongSpline`)))
  (`self.K2_SetActorRelativeTransform` (`KismetMathLibrary.MakeTransform` (`KismetMathLibrary.MakeVector` _returnvalue_x_2 _returnvalue_y_2 _returnvalue_z) _returnvalue_rotation))
  (if (>= (`self.DistanceAlongSpline`) (`SplineComponent.GetSplineLength` (`/Game/Task_05/BP_Trajectory.Spline` (`self.Trajectory`))))
    (set `self.DistanceAlongSpline` 0.0)))

(event `EnhancedInput|/Game/Basic/Input/IA_SpeedUp`
  (params (ActionValue :type Boolean) (ElapsedSeconds :type "Float (double-precision)") (TriggeredSeconds :type "Float (double-precision)") (InputAction :type "InputAction Object Reference" :default "/Game/Basic/Input/IA_SpeedUp.IA_SpeedUp"))
  ;[1 1 1] Changing speed of character
  (:`Triggered`
    (set `self.MoveSpeedAlongSpline` (+ (`self.MoveSpeedAlongSpline`) 200.0))))

(event `EnhancedInput|/Game/Basic/Input/IA_SpeedDown`
  (params (ActionValue :type Boolean) (ElapsedSeconds :type "Float (double-precision)") (TriggeredSeconds :type "Float (double-precision)") (InputAction :type "InputAction Object Reference" :default "/Game/Basic/Input/IA_SpeedDown.IA_SpeedDown"))
  ;[1 1 1] Changing speed of character
  (:`Triggered`
    (set `self.MoveSpeedAlongSpline` (- (`self.MoveSpeedAlongSpline`) 200.0))))

(event `EnhancedInput|/Game/Basic/Input/IA_LeftMouse`
  (params (ActionValue :type Boolean) (ElapsedSeconds :type "Float (double-precision)") (TriggeredSeconds :type "Float (double-precision)") (InputAction :type "InputAction Object Reference" :default "/Game/Basic/Input/IA_LeftMouse.IA_LeftMouse"))
  (bind _camera (`self.Camera`))
  (bind _prewievhitplace (`self.PrewievHitPlace`))
  (:`Triggered`
    (set `self.ThrowBallStartingPosition` (+ (`SceneComponent.K2_GetComponentLocation` _camera) (* (`SceneComponent.GetForwardVector` _camera) 300.0)))
    (set `self.FoundPreviewPlace` false)
    ;[1 1 1] Implementing projectile motion
    (for _array_element (`self.TimeArray`)
      (bind _returnvalue (`self.CalculateProjectilePosition` _array_element))
      (`KismetSystemLibrary.DrawDebugSphere` _returnvalue 12.0 12 (struct :`R` 1.0 :`A` 1.0))
      (if (not (`self.FoundPreviewPlace`))
        ;[1 1 1] Spawning preview mesh highly depends on amount of TimeArray elements. Position calculated based on previous and current point.
        (bind (_outhit _returnvalue_2) (`KismetSystemLibrary.SphereTraceSingle` (`self.ThrowBallStartingPosition`) _returnvalue 12.0 "TraceTypeQuery1"))
        (if _returnvalue_2
          (bind (_bblockinghit _binitialoverlap _time _distance _location _impactpoint _normal _impactnormal _physmat _hitactor _hitcomponent _hitbonename _bonename _hititem _elementindex _faceindex _tracestart) (`GameplayStatics.BreakHitResult` _outhit))
          (bind _returnvalue_3 (`|SpawnActorFromClass` "/Game/Task_05/BP_HitPlace.BP_HitPlace_C" (`KismetMathLibrary.MakeTransform` _location) "Undefined" "MultiplyWithRoot" self null))
          (set `self.PrewievHitPlace` _returnvalue_3)
          (set `self.FoundPreviewPlace` true)
          (else
            (set `self.ThrowBallStartingPosition` _tracestart)
            (`/Engine/EditorBlueprintResources/StandardMacros.IsValid` _prewievhitplace
              (:`Is Valid`
                (`self.K2_DestroyActor` _prewievhitplace))))))))
  (:`Completed`
    ;[1 1 1] Spawning BP_PhysicBall and setting Velocity
    (bind _returnvalue_4 (`|SpawnActorFromClass` "/Game/Task_05/BP_PhysicBall.BP_PhysicBall_C" (`KismetMathLibrary.MakeTransform` (`self.ThrowBallStartingPosition`)) "Undefined" "MultiplyWithRoot" self null))
    (`PrimitiveComponent.SetPhysicsLinearVelocity` (`/Game/Task_05/BP_PhysicBall.Sphere` _returnvalue_4) (* (`SceneComponent.GetForwardVector` (`self.Camera`)) (`self.PhysicBallStartingVelocity`)) false "None")))

(fn `CalculateProjectilePosition`
  (params (Time :type "Float (double-precision)"))
  (returns (ReturnValue :type "Vector Structure"))
  (bind _time (`local.Time`))
  (bind (_returnvalue_x _returnvalue_y _returnvalue_z) (`KismetMathLibrary.BreakVector` (* (`SceneComponent.GetForwardVector` (`self.Camera`)) (`self.PhysicBallStartingVelocity`))))
  (return (`KismetMathLibrary.MakeVector` (+ (.x (`self.ThrowBallStartingPosition`)) (* _returnvalue_x _time)) (+ (.y (`self.ThrowBallStartingPosition`)) (* _returnvalue_y _time)) (- (+ (.z (`self.ThrowBallStartingPosition`)) (* _returnvalue_z (`local.Time`))) (/ (* (`self.PhysicBallGravity`) (`KismetMathLibrary.Square` (`local.Time`))) 2.0)))))

(fn `UserConstructionScript`)