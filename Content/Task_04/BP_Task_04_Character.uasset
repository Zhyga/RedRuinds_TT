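; BP_Task_04_Character is a character Blueprint that exercises network replication of values on a UObject and creation of a dynamic component.
; BeginPlay shows a W_Helper widget, and Tick prints the StaticMeshComponent name and TestObject's three values.
; BP_ChangeValues changes TestObject directly on the server or through the object's own server RPC otherwise; a character-level alternative is left disconnected.
; CreateDynamicComponent forwards to CreateDynamicObject.
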(event `self.ReceiveBeginPlay`
  (`parent.ReceiveBeginPlay`)
  (bind _returnvalue (`|CreateWidget` "/Game/Task_04/Widgets/W_Helper.W_Helper_C"))
  (`UserWidget.AddToViewport` _returnvalue 0))

(event `self.ReceiveTick`
  (params (DeltaSeconds :type "Float (single-precision)"))
  (bind _testobject (`self.TestObject`))
  (`KismetSystemLibrary.PrintString` (`KismetSystemLibrary.GetDisplayName` (`self.StaticMeshComponent`)))
  (`/Engine/EditorBlueprintResources/StandardMacros.IsValid` _testobject
    (:`Is Valid`
      (`KismetSystemLibrary.PrintString` (`KismetTextLibrary.Conv_TextToString` (`|FormatText` "{a} \n{b} \n{c}" (`TestObject.value1` _testobject) (`TestObject.value2` _testobject) (`TestObject.value3` _testobject))) true true (struct :`R` 1.0 :`G` 0.165626 :`B` 0.20543 :`A` 1.0) 0.0))))

(event `BP_ChangeValues`
  (bind _testobject (`self.TestObject`))
  (if (`KismetSystemLibrary.IsServer`)
    ;[1 1 1] Replicate values using UObject
    (`TestObject.ChangeValues` _testobject)
    (else
      (`TestObject.RPC_Server_ChangeValues` _testobject))))

(event `CreateDynamicComponent`
  (`self.CreateDynamicObject`))

(fn `UserConstructionScript`)