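; Player character for Task 01 that detects interactable objects, toggles their text prompt and lets the player interact with them.
; Each tick, a debug-drawn Visibility trace runs from the mesh toward a point ahead of the camera, caching actors implementing BPI_Interact.
; On target change, an absolute dot-product alignment test against mesh forward decides whether the prompt shows.
; IA_Interact sends InteractMessage to the cached object.
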(event `self.ReceiveTick`
  (params (DeltaSeconds :type "Float (single-precision)"))
  (bind _camera (`self.Camera`))
  (bind _outhit (`KismetSystemLibrary.LineTraceSingle` :`Start` (`SceneComponent.K2_GetComponentLocation` (`self.Mesh`)) :`End` (+ (`SceneComponent.K2_GetComponentLocation` _camera) (* (`SceneComponent.GetForwardVector` _camera) 500.0)) :`TraceChannel` "TraceTypeQuery1" :`DrawDebugType` "ForOneFrame"))
  (bind (_bblockinghit _binitialoverlap _time _distance _location _impactpoint _normal _impactnormal _physmat _hitactor) (`GameplayStatics.BreakHitResult` _outhit))
  (if (!= (`self.InteractibleObject`) _hitactor)
    (if (`KismetSystemLibrary.DoesImplementInterface` _hitactor "/Game/Task_01/Blueprints/BPI_Interact.BPI_Interact_C")
      (bind _output_get (set `self.InteractibleObject` _hitactor))
      (if (`self.IsVisible` _output_get)
        (message `/Game/Task_01/Blueprints/BPI_Interact.ShowText` _output_get true)
        (else
          (message `/Game/Task_01/Blueprints/BPI_Interact.ShowText` _output_get false)))
      (else
        (message `/Game/Task_01/Blueprints/BPI_Interact.ShowText` (`self.InteractibleObject`) false)
        (set `self.InteractibleObject` null)))))

(event `EnhancedInput|/Game/Basic/Input/IA_Interact`
  (params (ActionValue :type Boolean) (ElapsedSeconds :type "Float (double-precision)") (TriggeredSeconds :type "Float (double-precision)") (InputAction :type "InputAction Object Reference" :default "/Game/Basic/Input/IA_Interact.IA_Interact"))
  (bind _interactibleobject (`self.InteractibleObject`))
  (:`Triggered`
    (`/Engine/EditorBlueprintResources/StandardMacros.IsValid` _interactibleobject
      (:`Is Valid`
        (message `/Game/Task_01/Blueprints/BPI_Interact.Interact` _interactibleobject)))))

(fn `IsVisible`
  (params (Target :type "Actor Object Reference"))
  (returns (Visible :type Boolean))
  (return (>= (`KismetMathLibrary.Abs` (`KismetMathLibrary.Dot_VectorVector` (`KismetMathLibrary.GetForwardVector` (`KismetMathLibrary.FindLookAtRotation` (`self.K2_GetActorLocation` Target) (`self.K2_GetActorLocation`))) (`SceneComponent.GetForwardVector` (`self.Mesh`)))) 0.7)))

(fn `UserConstructionScript`)