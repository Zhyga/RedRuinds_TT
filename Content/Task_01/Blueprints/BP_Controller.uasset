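; BP_Controller is a player controller Blueprint that sets up input and the HUD when play begins.
; BeginPlay calls two collapsed graphs in turn: one adds the IMC_Input mapping context to the Enhanced Input local player subsystem.
; The other creates a HUD widget owned by the controller and adds it to the viewport.
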(event `self.ReceiveBeginPlay`
  (`EnhancedInputSubsystemInterface.AddMappingContext` (subsystem `EnhancedInputLocalPlayerSubsystem`) "/Game/Basic/Input/IMC_Input.IMC_Input" 0 (struct))
  (bind _returnvalue (`|CreateWidget` "/Game/Task_01/Widgets/W_HUD.W_HUD_C" self))
  (`UserWidget.AddToViewport` _returnvalue 0))

(fn `UserConstructionScript`)