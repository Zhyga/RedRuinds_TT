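; BP_Task_01_Actor is an interactable task actor with a sphere, a marker widget and an interaction text.
; On BeginPlay it casts the marker widget to W_Marker and binds itself to it.
; Interact swaps the sphere's material once, guarded by an Activated flag.
; ShowDescription toggles the interaction text's visibility.
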(event `self.ReceiveBeginPlay`
  (bind _asw_marker (cast `/Game/Task_01/Widgets/W_Marker` (`WidgetComponent.GetWidget` (`self.Marker`))))
  (set `/Game/Task_01/Widgets/W_Marker.BindedActor` self _asw_marker))

(event `/Game/Task_01/Blueprints/BPI_Interact.Interact`
  (if (not (`self.bActivated`))
    (`PrimitiveComponent.SetMaterial` (`self.Sphere`) 0 "/Engine/MapTemplates/Materials/BasicAsset01.BasicAsset01")
    (set `self.bActivated` true)))

(event `/Game/Task_01/Blueprints/BPI_Interact.ShowDescription`
  (params (bShow :type Boolean))
  (`SceneComponent.SetVisibility` (`self.InteractionText`) bShow false))

(fn `UserConstructionScript`)