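; Steering-behavior agent that seeks the level's BP_Task_06_Target while avoiding obstacles and other agents of its class.
; Each Tick sums clamped seek, line-trace avoidance ahead along velocity, and distance-weighted separation from agents cached at BeginPlay.
; The result updates a speed-clamped velocity fed to FloatingPawnMovement, with rotation following velocity at a 90-degree pitch offset.
; FleeSteering and the cached StaticMeshActor list are unused.
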(event `self.ReceiveBeginPlay`
  (bind _returnvalue (`GameplayStatics.GetActorOfClass` "/Game/Task_06/BP_Task_06_Target.BP_Task_06_Target_C"))
  (set `self.Target` _returnvalue)
  (bind _outactors (`GameplayStatics.GetAllActorsOfClass` "BP_Task_06_Actor_C"))
  (set `self.Actors` _outactors)
  (bind _outactors_2 (`GameplayStatics.GetAllActorsOfClass` "/Script/Engine.StaticMeshActor"))
  (set `self.StaticMeshes` _outactors_2))

(event `self.ReceiveTick`
  (params (DeltaSeconds :type "Float (single-precision)"))
  (bind _returnvalue (`self.K2_GetActorLocation`))
  (bind (_returnvalue_roll _returnvalue_pitch _returnvalue_yaw) (`KismetMathLibrary.BreakRotator` (`KismetMathLibrary.FindLookAtRotation` _returnvalue (+ _returnvalue (`self.Velocity`)))))
  (`self.K2_SetActorRotation` (`KismetMathLibrary.MakeRotator` _returnvalue_roll (+ _returnvalue_pitch 90.0) _returnvalue_yaw))
  (bind _output_get (set `self.Steering` (0.0 0.0 0.0)))
  (set `self.Steering` (+ (`KismetMathLibrary.Vector_ClampSizeMax` (`self.SeekSteering` (`self.K2_GetActorLocation` (`self.Target`)) 1.0) (`self.MaxForce`)) _output_get (`self.CalculateAvoidanceForce`) (`self.SeparationSteering`)))
  (bind _output_get_2 (set `self.Velocity` (`KismetMathLibrary.Vector_ClampSizeMax` (+ (`self.Steering`) (`self.Velocity`)) (`self.MaxSpeed`))))
  (`PawnMovementComponent.AddInputVector` (`self.FloatingPawnMovement`) _output_get_2 false))

(fn `CalculateAheadVector`
  (returns (AheadVector :type "Vector Structure"))
  (return (+ (`self.K2_GetActorLocation`) (* (`KismetMathLibrary.Normal` (`self.Velocity`)) (`self.DistanceAhead`)))))

(fn `CalculateAvoidanceForce`
  (returns (AvoidanceForce :type "Vector Structure"))
  (bind (_outhit _returnvalue) (`KismetSystemLibrary.LineTraceSingle` (`self.K2_GetActorLocation`) (`self.CalculateAheadVector`) "TraceTypeQuery1"))
  (if _returnvalue
    (return (* (`KismetMathLibrary.Normal` (- (`self.CalculateAheadVector`) (`self.K2_GetActorLocation` (`.HitActor` (`GameplayStatics.BreakHitResult` _outhit))))) (`self.AvoidForce`)))
    (else
      (return (0.0 0.0 0.0)))))

(fn `FleeSteering`
  (params (ActorPosition :type "Vector Structure"))
  (returns (NewSteering :type "Vector Structure"))
  (locals (DesiredVelocity :type "Vector Structure"))
  (bind _output_get (set `local.DesiredVelocity` (* (`KismetMathLibrary.GetDirectionUnitVector` ActorPosition (`self.K2_GetActorLocation`)) (`self.MaxForce`))))
  (return (- _output_get (`self.Velocity`))))

(fn `SeekSteering`
  (params (TargetPosition :type "Vector Structure") (Weight :type "Float (double-precision)"))
  (returns (Steering :type "Vector Structure"))
  (locals (DesiredVelocity :type "Vector Structure"))
  (bind _output_get (set `local.DesiredVelocity` (* (`KismetMathLibrary.GetDirectionUnitVector` (`self.K2_GetActorLocation`) TargetPosition) (`self.MaxSpeed`))))
  (return (- _output_get (`self.Velocity`))))

(fn `SeparationSteering`
  (returns (SeparationSteering :type "Vector Structure"))
  (locals (SeparetionVector :type "Vector Structure") (Count :type "Float (double-precision)") (VecTo :type "Vector Structure"))
  (bind _separationdistance (`self.SeparationDistance`))
  (for _array_element (`self.Actors`)
    (if (!= _array_element self)
      (bind _output_get (set `local.VecTo` (- (`self.K2_GetActorLocation`) (`self.K2_GetActorLocation` _array_element))))
      (set `local.VecTo` (* (`local.VecTo`) (- 1.0 (/ (`KismetMathLibrary.FMin` (`KismetMathLibrary.VSize` _output_get) _separationdistance) _separationdistance))))
      (set `local.SeparetionVector` (+ (`local.SeparetionVector`) (`local.VecTo`)))
      (`/Engine/EditorBlueprintResources/StandardMacros.IncrementFloat` (`local.Count`))))
  (if (> (`local.Count`) 0.0)
    (return (`KismetMathLibrary.Vector_ClampSizeMax` (`local.SeparetionVector`) (`self.MaxForce`)))
    (else
      (return (0.0 0.0 0.0)))))

(fn `UserConstructionScript`)